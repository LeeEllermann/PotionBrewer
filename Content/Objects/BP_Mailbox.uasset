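; Interactable mailbox that hands out a fixed sequence of quests through its QuestGiverComponent while a next quest is available.
; NextQuest starts a looping timer that, on completion, advances the quest counter, loads the matching data table row and shows both the prompt widget and a HUD notification.
; When the counter passes the third quest, it disables further quests and opens the WB_LastPotion screen with mouse input.
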(event `self.ReceiveBeginPlay`
  (`self.Update Quest Row` "10001"))

(event `/Game/Interfaces/I_HUD-Interface.Hide Quest Indicator`
  (`SceneComponent.SetVisibility` (`self.Widget Prompt`) false false))

(event `/Game/Interfaces/I_HUD-Interface.Show Quest Indicator`
  (`SceneComponent.SetVisibility` (`self.Widget Prompt`) true false))

(event `/Game/Interfaces/I_InteractInterface.Next Quest`
  (`self.Start Timer`))

(event `Start Timer`
  (bind _returnvalue (`KismetSystemLibrary.K2_SetTimer` null "New Quest Timer" (`self.Timer Speed`) true)))

(event `Stop Timer`
  (bind _returnvalue (`GameplayStatics.GetPlayerController` 0))
  (`KismetSystemLibrary.K2_ClearAndInvalidateTimerHandle` (stale `Start Timer` _returnvalue))
  (set `self.Current Timer` 0.0)
  (if (`self.IsNextQuestAvailable`)
    (bind _result (`/Engine/EditorBlueprintResources/StandardMacros.IncrementInt` (`self.ActiveQuestCounter`))
      (:`  `
        (switch `int` _result
          (:`Default`
            (set `self.IsNextQuestAvailable` false)
            (bind _returnvalue_2 (`|CreateWidget` "/Game/Widgets/WB_LastPotion.WB_LastPotion_C"))
            (`UserWidget.AddToViewport` _returnvalue_2 0)
            (`WidgetBlueprintLibrary.SetInputMode_GameAndUIEx` _returnvalue _returnvalue_2)
            (set `PlayerController.bShowMouseCursor` true _returnvalue))
          (:`1`
            (`self.Update Quest Row` "10001")
            (bind _foundwidgets (`WidgetBlueprintLibrary.GetAllWidgetsWithInterface` "/Game/Interfaces/I_HUD-Interface.I_HUD-Interface_C" :!label _label))
            (for _array_element _foundwidgets
              (message `/Game/Interfaces/I_HUD-Interface.Show Quest Indicator` _array_element))
            (`/Game/Interfaces/I_HUD-Interface.Show Quest Indicator`))
          (:`2`
            (`self.Update Quest Row` "10002")
            (goto _label))
          (:`3`
            (`self.Update Quest Row` "10003")
            (goto _label)))))))

(fn `InteractWith`
  (params (`Player Character` :type "/Game/Blueprints/BP_ThirdPersonCharacter Object Reference"))
  (returns (`Interaction ID` :type String))
  (if (`self.IsNextQuestAvailable`)
    (bind _interaction_id (`/Game/Interfaces/I_InteractInterface.InteractWith` (`self.QuestGiver_Component`) `Player Character`))
    (return _interaction_id)))

(fn `LookAt`
  (returns (Message :type Text))
  (return "Mailbox"))

(fn `New Quest Timer`
  (if (< (`self.Current Timer`) (`self.Max Timer`))
    (set `self.Current Timer` (+ (`self.Current Timer`) 0.1))
    (else
      (`self.Stop Timer`))))

(fn `Update Quest Row`
  (params (`Row Name` :type Name))
  (set `/Game/QuestSystem/QuestGiver_Component.Quest Data` (make `DataTableRowHandle` "/Game/QuestSystem/QuestData.QuestData" `Row Name`) (`self.QuestGiver_Component`)))

(fn `UserConstructionScript`)