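; BP_CauldronArea is an interactable cauldron where the player brews and collects a potion.
; StartCauldronArea resets it and shows its progress bar, then interacting moves a state machine from brewing to collection, returning objective IDs.
; A looping timer advances progress until the potion is ready, while Tick broadcasts that value to all I_WidgetInterface widgets.
; Starting a brew also notifies those widgets and hides ingredient indicators on I_InteractInterface actors.
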(event `self.ReceiveBeginPlay`
  (`SceneComponent.SetVisibility` (`self.Progress Bar Widget`) false false))

(event `self.ReceiveTick`
  (params (DeltaSeconds :type "Float (single-precision)"))
  (bind _foundwidgets (`WidgetBlueprintLibrary.GetAllWidgetsWithInterface` "/Game/Interfaces/I_WidgetInterface.I_WidgetInterface_C"))
  (for _array_element _foundwidgets
    (message `/Game/Interfaces/I_WidgetInterface.PotionProgressUpdated` _array_element (`self.CurrentPotionProgress`))))

(event `Start Potion Timer`
  (bind _returnvalue (`KismetSystemLibrary.K2_SetTimer` null "PotionTimer" (`self.FillSpeed`) true)))

(event `Stop Potion Timer`
  (`KismetSystemLibrary.K2_ClearAndInvalidateTimerHandle` (stale `Start Potion Timer` _returnvalue)))

(event `/Game/Interfaces/I_InteractInterface.Start Cauldron Area`
  (set `self.CurrentPotionState` "NewEnumerator3")
  (`SceneComponent.SetVisibility` (`self.Progress Bar Widget`) true false)
  (bind _foundwidgets (`WidgetBlueprintLibrary.GetAllWidgetsWithInterface` "/Game/Interfaces/I_WidgetInterface.I_WidgetInterface_C"))
  (for _array_element _foundwidgets
    (message `/Game/Interfaces/I_WidgetInterface.Restart Potion Process` _array_element))
  (set `self.CurrentPotionProgress` 0.0))

(fn `InteractWith`
  (params (`Player Character` :type "/Game/Blueprints/BP_ThirdPersonCharacter Object Reference"))
  (returns (`Interaction ID` :type String))
  (switch `/Game/Interfaces/E_PotionState` (`self.CurrentPotionState`)
    (:`NewEnumerator0`
      (return (`self.Objective ID`)))
    (:`NewEnumerator3`
      (`self.Start Potion`)
      (set `self.CurrentPotionState` "NewEnumerator1")
      (return (`self.Objective ID`)))
    (:`NewEnumerator1`
      (return (`self.Objective ID`)))
    (:`NewEnumerator2`
      (`/Game/Libraries/FL_Misc.Print Debug Message` "Collecting Potion" "NewEnumerator2" 20.0)
      (`SceneComponent.SetVisibility` (`self.Progress Bar Widget`) false false)
      (set `self.CurrentPotionState` "NewEnumerator0")
      (return (`self.Objective ID Potion`)))))

(fn `LookAt`
  (returns (Message :type Text))
  (return "Cauldron"))

(fn `PotionTimer`
  (if (< (`self.CurrentPotionProgress`) (`self.MaxPotionTime`))
    (set `self.CurrentPotionProgress` (+ (`self.CurrentPotionProgress`) 0.1))
    (else
      (`self.Stop Potion Timer`)
      (set `self.CurrentPotionState` "NewEnumerator2"))))

(fn `Start Potion`
  (bind _foundwidgets (`WidgetBlueprintLibrary.GetAllWidgetsWithInterface` "/Game/Interfaces/I_WidgetInterface.I_WidgetInterface_C"))
  (for _array_element _foundwidgets
    (message `/Game/Interfaces/I_WidgetInterface.StartPotionBrewing` _array_element)
    (`self.Start Potion Timer`))
  (bind _outactors (`GameplayStatics.GetAllActorsWithInterface` "/Game/Interfaces/I_InteractInterface.I_InteractInterface_C"))
  (for _array_element_2 _outactors
    (message `/Game/Interfaces/I_InteractInterface.Hide All Ingredient Indicators` _array_element_2)))

(fn `UserConstructionScript`)