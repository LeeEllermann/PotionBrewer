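; Base quest Blueprint that tracks objective progress for the current stage of a quest.
; On BeginPlay it loads the QuestID row from the QuestData table, zeroes a progress map keyed by objective ID and binds to the player inventory's objective event.
; Positive changes count only for tracked objectives below their quantity, then update the Completed flag.
; Other changes apply without rechecking completion, and nothing here advances the stage.
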(event `self.ReceiveBeginPlay`
  (`self.Get Quest Details`)
  (bind _all_complete (`self.Are All Objectives Complete`))
  (set `self.Completed` _all_complete)
  (add `/Game/Inventory/InventoryComponent.On Objective ID Called` (`/Game/Blueprints/BP_ThirdPersonCharacter.Inventory` (`/Game/Libraries/CommonFunctionLibrary_RyanLaley.Get My Player Character`)) (`|CreateDelegate` :!event `On Objective ID Heard`)))

(fn `Are All Objectives Complete`
  (returns (`All Complete` :type Boolean))
  (locals (Local_AllComplete :type Boolean :default true))
  (for _array_element (`.Objectives_15_CA101DCD438ADD271CBE13A24B596670` (break `/Game/QuestSystem/F_StageDetails` (`self.Current Stage Details`)))
    (bind (_objectivename _description _type _objectiveid) (break `/Game/QuestSystem/F_ObjectiveDetails` _array_element))
    (if (not (>= (`BlueprintMapLibrary.Map_Find` (`self.Current Objective Progress`) _objectiveid) (`.Quantity_12_5AEA6C524C7A97607881BAB35DD7006E` (break `/Game/QuestSystem/F_ObjectiveDetails` (`self.Get Objective Data By ID` _objectiveid)))))
      (bind _output_get (set `local.Local_AllComplete` false))
      (return _output_get)))
  (return (`local.Local_AllComplete`)))

(fn `Get Objective Data By ID`
  (params (`Objective ID` :type String))
  (returns (`Array Element` :type "/Game/QuestSystem/F_ObjectiveDetails Structure"))
  (for _array_element (`.Objectives_15_CA101DCD438ADD271CBE13A24B596670` (break `/Game/QuestSystem/F_StageDetails` (`self.Current Stage Details`)))
    (if (`KismetStringLibrary.EqualEqual_StrStr` (`.ObjectiveID_9_1672035049B805BEC8F9F5AFB091FE7D` (break `/Game/QuestSystem/F_ObjectiveDetails` _array_element)) `Objective ID`)
      (return _array_element))))

(fn `Get Quest Details`
  (bind _returnvalue (`|GetDataTableRow` "/Game/QuestSystem/QuestData.QuestData" (`self.QuestID`))
    (:`then`
      (bind _output_get (set `self.QuestDetails` _returnvalue))
      (bind _output_get_2 (set `self.Current Stage Details` (`|GetArrayItem` (`.Stages_15_20F286434599C52D6B0044A466E83CE7` (break `/Game/QuestSystem/F_QuestDetails` _output_get)) (`self.Current Stage`))))
      (`BlueprintMapLibrary.Map_Clear` (`self.Current Objective Progress`))
      (for _array_element (`.Objectives_15_CA101DCD438ADD271CBE13A24B596670` (break `/Game/QuestSystem/F_StageDetails` _output_get_2))
        (`BlueprintMapLibrary.Map_Add` (`self.Current Objective Progress`) (`.ObjectiveID_9_1672035049B805BEC8F9F5AFB091FE7D` (break `/Game/QuestSystem/F_ObjectiveDetails` _array_element)))))))

(fn `Is Objective Complete`
  (params (`Objective ID` :type String))
  (bind ((`Description_4_C08EECB5492816C94040FEA8866D47F5` _description) (`Quantity_12_5AEA6C524C7A97607881BAB35DD7006E` _quantity)) (break `/Game/QuestSystem/F_ObjectiveDetails` (`self.Get Objective Data By ID` `Objective ID`)))
  (if (>= (`BlueprintMapLibrary.Map_Find` (`self.Current Objective Progress`) (`local.Objective ID`)) _quantity)
    (`/Game/Libraries/FL_Misc.Print Debug Message` (`KismetStringLibrary.Concat_StrStr` "Objective Complete: " (`KismetTextLibrary.Conv_TextToString` _description)) "NewEnumerator3" 10.0)
    (bind _all_complete (`self.Are All Objectives Complete`))
    (set `self.Completed` _all_complete)))

(fn `On Objective ID Heard`
  (params (`Objective ID` :type String) (Value :type Integer :default 1))
  (bind (_value _returnvalue) (`BlueprintMapLibrary.Map_Find` (`self.Current Objective Progress`) (`local.Objective ID`)))
  (if (> (`KismetMathLibrary.SignOfInteger` Value) 0)
    (if _returnvalue
      (if (< _value (`.Quantity_12_5AEA6C524C7A97607881BAB35DD7006E` (break `/Game/QuestSystem/F_ObjectiveDetails` (`self.Get Objective Data By ID` (`local.Objective ID`)))))
        (`BlueprintMapLibrary.Map_Add` (`self.Current Objective Progress`) (`local.Objective ID`) (+ _value (`local.Value`)))
        (`self.Is Objective Complete` (`local.Objective ID`))
        (return))
      (else
        (return)))
    (else
      (`BlueprintMapLibrary.Map_Add` (`self.Current Objective Progress`) (`local.Objective ID`) (+ (`BlueprintMapLibrary.Map_Find` (`self.Current Objective Progress`) (`local.Objective ID`)) (`local.Value`)))
      (return))))

(fn `UserConstructionScript`)